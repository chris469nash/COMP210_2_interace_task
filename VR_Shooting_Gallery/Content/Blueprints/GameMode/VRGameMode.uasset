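; VR game mode that runs a wave-based enemy game from start to game over.
; StartGame resets the score and hides the in-game menu, which reappears once all waves have spawned and the last delay ends.
; Before each wave, a timeline animates the floor grid colour through a material parameter collection.
; Each wave shuffles interface-discovered spawners, triggers the configured count, then schedules the next wave by timer.
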(event Custom|HandleGameOver
  (bind _ingamemenuref (Variables|Default|GetInGameMenuRef))
  (Rendering|SetActorHiddenInGame _ingamemenuref false)
  (Collision|SetActorEnableCollision _ingamemenuref true))

(event Custom|HandleSpawningNewWave
  (if (> (Variables|Default|GetCurrentWaveNumber) (Utilities|Array|LastIndex (Variables|Default|GetEnemiesPerWave)))
    (CallFunction|HandleGameOver)
    (else
      (bind _newcolour (Timeline|ColourChange PlayFromStart)
        (:Update
          (Rendering|Material|SetVectorParameterValue "/Game/Materials/FloorMatMPC.FloorMatMPC" "GridColour" _newcolour :!class /Script/Engine.KismetMaterialLibrary))
        (:Finished
          (CallFunction|SpawnEnemyWave))))))

(event EventBeginPlay
  (bind _outactors (Actor|GetAllActorswithInterface "/Game/Blueprints/Interfaces/BPI_EnemySpawner.BPI_EnemySpawner_C"))
  (Variables|Default|SetEnemySpawners _outactors)
  (bind _outactors_2 (Actor|GetAllActorswithInterface "/Game/Blueprints/Interfaces/BPI_InGameMenuBP.BPI_InGameMenuBP_C"))
  (Variables|Default|SetInGameMenuRef (Utilities|Array|Get(acopy) _outactors_2)))

(event EventStartGame
  (bind _ingamemenuref (Variables|Default|GetInGameMenuRef))
  (Class|BPIPlayer|ResetScore(Message) (Game|Player|GetPlayerPawn 0))
  (Variables|Default|SetCurrentWaveNumber 0)
  (Rendering|SetActorHiddenInGame _ingamemenuref true)
  (Collision|SetActorEnableCollision _ingamemenuref false)
  (CallFunction|HandleSpawningNewWave))

(fn ConstructionScript)

(fn SpawnEnemyWave
  (Utilities|Array|Shuffle (Variables|Default|GetEnemySpawners))
  (for _index (range 0 (- (Utilities|Array|Get(acopy) (Variables|Default|GetEnemiesPerWave) (Variables|Default|GetCurrentWaveNumber)) 1))
    (Class|BPIEnemySpawner|HandleSpawnEnemy(Message) (Utilities|Array|Get(acopy) (Variables|Default|GetEnemySpawners) _index)))
  (Math|Integer|IncrementInt (Variables|Default|GetCurrentWaveNumber)
    (:%20%20
      (Utilities|Time|SetTimerbyFunctionName 0 "HandleSpawningNewWave" (Variables|Default|GetDelayPerWave)))))