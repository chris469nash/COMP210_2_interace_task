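; VRGameMode is a game mode that runs timed waves of enemy spawns.
; On BeginPlay it gathers every actor implementing BPI_EnemySpawner and starts the first wave.
; Each wave shuffles the spawners and sends a spawn message to as many as that wave's EnemiesPerWave entry specifies, so each fires once.
; SpawnEnemyWave then re-schedules itself by timer after DelayPerWave, stopping once the wave list runs out.
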(event EventBeginPlay
  (bind _outactors (Actor|GetAllActorswithInterface "/Game/Blueprints/Interfaces/BPI_EnemySpawner.BPI_EnemySpawner_C"))
  (Variables|Default|SetEnemySpawners _outactors)
  (CallFunction|SpawnEnemyWave))

(fn ConstructionScript)

(fn SpawnEnemyWave
  (if (not (> (Variables|Default|GetCurrentWaveNumber) (Utilities|Array|LastIndex (Variables|Default|GetEnemiesPerWave))))
    (Utilities|Array|Shuffle (Variables|Default|GetEnemySpawners))
    (for _index (range 0 (- (Utilities|Array|Get(acopy) (Variables|Default|GetEnemiesPerWave) (Variables|Default|GetCurrentWaveNumber)) 1))
      (Class|BPIEnemySpawner|HandleSpawnEnemy(Message) (Utilities|Array|Get(acopy) (Variables|Default|GetEnemySpawners) _index)))
    (Math|Integer|IncrementInt (Variables|Default|GetCurrentWaveNumber)
      (:%20%20
        (Utilities|Time|SetTimerbyFunctionName 0 "SpawnEnemyWave" (Variables|Default|GetDelayPerWave))))))